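; Player controller for a tile-grid game that shows the cursor, creates the HUD and sends join and move requests.
; Select clicks trace under the cursor and convert the hit to a tile, either appended to Path as a byte index in MoveMode or broadcast through OnSelectTile.
; SendMove executes MSSTMove with the Path and clears it; JoinGame executes MSSTJoinGame at position 0,0.
; GetXandY is an unimplemented stub returning zeros.
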(event `InputAction|SendMove`
  (params (Key :type "Key Structure"))
  (:`Pressed`
    (`MS_ST_BytesBasedBase.Execute` (subsystem `MS_ST_Move`) (`self.Path`))
    (`KismetArrayLibrary.Array_Clear` (`.value` (break `C_ST_Bytes` (`self.Path`))))))

(event `InputAction|Select`
  (params (Key :type "Key Structure"))
  (bind _hitresult (`self.GetHitResultUnderCursorByChannel` "TraceTypeQuery1"))
  (:`Pressed`
    (if (`GameplayStatics.BreakHitResult` _hitresult)
      (bind (_x _y) (`self.GetNodeAddress` (`.ImpactPoint` (`GameplayStatics.BreakHitResult` _hitresult))))
      (if (`self.MoveMode`)
        (`KismetArrayLibrary.Array_Add` (`.value` (break `C_ST_Bytes` (`self.Path`))) (`KismetMathLibrary.Conv_IntToByte` (+ _x (* _y (`self.Width`)))))
        (else
          (`self.OnSelectTile` _x _y))))))

(event `self.ReceiveBeginPlay`
  (set `self.bShowMouseCursor` true)
  (bind _returnvalue (`|CreateWidget` "/Game/Blueprints/UI/HUD/BP_HUD.BP_HUD_C" self))
  (`UserWidget.AddToViewport` _returnvalue 0))

(event `InputAction|JoinGame`
  (params (Key :type "Key Structure"))
  (:`Pressed`
    (`MS_ST_PositionBasedBase.Execute` (subsystem `MS_ST_JoinGame`) (make `C_ST_Position` 0))))

(fn `GetNodeAddress`
  (params (WorldLocation :type "Vector Structure"))
  (returns (x :type Integer) (y :type Integer))
  (locals (NodeAddress :type Integer))
  (return (`KismetMathLibrary.FTrunc` (/ (+ WorldLocation_X 100.0) (`self.TileSize`))) (`KismetMathLibrary.FTrunc` (/ (+ WorldLocation_Y 100.0) (`self.TileSize`)))))

(fn `GetWorldLocation`
  (params (x :type Integer) (y :type Integer))
  (returns (WorldLocation :type "Vector Structure") (WorldLocation_X :type "Float (double-precision)") (WorldLocation_Y :type "Float (double-precision)") (WorldLocation_Z :type "Float (double-precision)"))
  (bind (_returnvalue_x _returnvalue_y _returnvalue_z) (`KismetMathLibrary.BreakVector` (`self.K2_GetActorLocation`)))
  (return (`KismetMathLibrary.MakeVector` (* x (`self.TileSize`)) (* y (`self.TileSize`)) _returnvalue_z) 0.0 0.0 0.0))

(fn `GetXandY`
  (params (Address :type Integer))
  (returns (X :type Integer) (Y :type Integer))
  (return 0 0))

(fn `UserConstructionScript`)